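; Base enemy character for a basic AI system, delegating damage and health to a BPCDamageSystem component.
; The construction script binds death and damage-response events, with death playing a sound and destroying the actor.
; Functions expose health, patrol object and walk speed by movement state, while mana, stamina, heal, range and token functions return placeholder values.
; Attack events branch by melee, range or explosion type but only print messages for child classes to replace.
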(event Custom|Death
  (params (DamageResponse :type E_DeathResponse%20Enum :default "NewEnumerator0"))
  (Audio|PlaySound2D "/Game/seranUI/Star_Wars_Death_Noise___mp3cut_net_.Star_Wars_Death_Noise___mp3cut_net_" 1.0 1.0 0.0 0 0)
  (Development|PrintString "Hello")
  (Actor|DestroyActor))

(event Custom|DamageResponse
  (params (Damage :type E_DamageResponsee%20Enum :default "NewEnumerator0"))
  (Development|PrintString "damage"))

(event EventTakeDamage
  (params (AboutDamage :type S%20Damage%20AMK%20Structure))
  (Default|TakeDamage (Variables|Default|GetBPC_DamageSystem) AboutDamage)
  (Development|PrintString "sadasdasdas" true true "(R=1.000000,G=0.177770,B=0.000000,A=1.000000)"))

(event EventEnemyAttack
  (params (enemyAttackType :type E_AttackType%20Enum :default "NewEnumerator0"))
  (switch Utilities|FlowControl|Switch|SwitchonE_AttackType enemyAttackType
    (:NewEnumerator0
      (Development|PrintString "addMeleeChildObject"))
    (:NewEnumerator1
      (Development|PrintString "addRangeChildObject"))
    (:NewEnumerator2
      (Development|PrintString "addExplosiveChildObject"))))

(fn ConstructionScript
  (EventDispatchers|BindEventtoDeath (Variables|Default|GetBPC_DamageSystem) (EventDispatchers|CreateEvent :!event Custom|Death))
  (EventDispatchers|BindEventtoDamageResponse (Variables|Default|GetBPC_DamageSystem) (EventDispatchers|CreateEvent :!event Custom|DamageResponse)))

(fn GetCurrentHealth
  (return (Variables|/Game/MyThing_DamageSystem/DamageSystemByMe/BPC_DamageSystem.BPC_DamageSystem_C|GetcurrentHealth (Variables|Default|GetBPC_DamageSystem))))

(fn GetCurrentMana
  (return 0.0))

(fn GetCurrentStamina
  (return 0.0))

(fn GetMaxHealth
  (return (Variables|/Game/MyThing_DamageSystem/DamageSystemByMe/BPC_DamageSystem.BPC_DamageSystem_C|GetmaxHealth (Variables|Default|GetBPC_DamageSystem))))

(fn GetMaxMana
  (return 0.0))

(fn GetMaxStamina
  (return 0.0))

(fn Heal
  (params (amountOfHeal :type Float%20%28double-precision%29))
  (return 0.0))

(fn IsDead
  (return (Variables|Default|GetIs%20Deadd)))

(fn Patrol
  (return (Variables|Default|GetpatroObject)))

(fn SetMovementSpeed
  (params (movementSpeedEnum :type E_MovementSpeed%20Enum :default "NewEnumerator0"))
  (bind _output_get (Variables|/Script/Engine.CharacterMovementComponent|SetMaxWalkSpeed (Variables|Character|GetCharacterMovement) (Utilities|Select :Index movementSpeedEnum :NewEnumerator0 0.0 :NewEnumerator1 3e+02 :NewEnumerator2 6e+02)))
  (return _output_get))

(fn SetRange
  (return (Utilities|Struct|MakeS_Range 0.0 0.0)))

(fn TookToken
  (params (amountOfToken :type Integer))
  (return false))