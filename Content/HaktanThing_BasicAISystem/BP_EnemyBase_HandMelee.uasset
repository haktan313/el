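; Melee enemy variant in the basic AI system that attacks the player with a montage and reports completion or interruption through the attack dispatcher.
; AttackTraceStart runs a looping timer that sphere-traces between two mesh sockets, with debug drawing on.
; A DoOnce gate limits damage on Player-tagged actors, and AttackTraceStop clears the timer and resets it.
; Helper functions set walk speed per movement state and supply attack and defense radii.
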(event Custom|AttackTraceStart
  (bind _returnvalue (Utilities|Time|SetTimerbyEvent (delegate Custom|Trace) 0.1 true))
  (Variables|Default|SetNewVar _returnvalue))

(event Custom|Trace
  (bind (_outhit _returnvalue) (Collision|SphereTraceByChannel (Transformation|GetSocketLocation (Variables|Character|GetMesh) "attack") (Transformation|GetSocketLocation (Variables|Character|GetMesh) "end") 12.0 "TraceTypeQuery2" false (Utilities|Array|MakeArray self) "ForDuration" true "(R=1.000000,G=0.000000,B=0.000000,A=1.000000)" "(R=0.000000,G=1.000000,B=0.000000,A=1.000000)" 0.0))
  (if _returnvalue
    (bind _output_get (Variables|Default|SetHit%20Actor (.HitActor (Collision|BreakHitResult _outhit))))
    (if (Actor|ActorHasTag _output_get "Player")
      (Utilities|FlowControl|DoOnce false
        (:Completed
          (Class|BPIStats|TakeDamage(Message) (Variables|Default|GetHit%20Actor) (Utilities|Struct|MakeS_DamageAMK 1e+01 "NewEnumerator0" "NewEnumerator0"))
          (CallFunction|AttackTraceStop))))))

(event Custom|AttackTraceStop
  (Utilities|Time|ClearandInvalidateTimerbyHandle (Variables|Default|GetNewVar))
  (Utilities|FlowControl|DoOnce false) ; enters at Reset
)

(event Collision|EventActorBeginOverlap
  (params (OtherActor :type Actor%20Object%20Reference)))

(event EventTick
  (params (DeltaSeconds :type Float%20%28single-precision%29)))

(event EventEnemyAttack
  (params (enemyAttackType :type E_AttackType%20Enum :default "NewEnumerator0"))
  (switch Utilities|FlowControl|Switch|SwitchonE_AttackType enemyAttackType
    (:NewEnumerator0
      (Animation|Montage|PlayMontage (Variables|Character|GetMesh) "/Game/NewFolder/kickimdat_Anim_2_Montage.kickimdat_Anim_2_Montage" 1.2 0.0 "start"
        (:OnCompleted
          _)
        (:OnInterrupted
          _))
      (Default|CallAttackDispatcher))))

(event EventBeginPlay)

(fn ConstructionScript
  (|CallParentFunction))

(fn SetMovementSpeed
  (params (movementSpeedEnum :type E_MovementSpeed%20Enum :default "NewEnumerator0"))
  (bind _output_get (Variables|/Script/Engine.CharacterMovementComponent|SetMaxWalkSpeed (Variables|Character|GetCharacterMovement) (Utilities|Select :Index movementSpeedEnum :NewEnumerator0 0.0 :NewEnumerator1 5e+02 :NewEnumerator2 6e+02)))
  (return _output_get))

(fn SetRange
  (return (Utilities|Struct|MakeS_Range 225.0 225.0)))