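; Actor component in the basic AI system that holds a counted pool of tokens for callers to take and return.
; TookToken deducts the requested amount and returns true when CurrentToken covers it, otherwise returns false and leaves the count unchanged.
; GiveTokenBack adds the amount back with no upper limit check.
; The event graph is empty, so the count changes only through function calls.
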(event EventBeginPlay)

(event EventTick
  (params (DeltaSeconds :type Float%20%28single-precision%29)))

(fn TookToken
  (params (amountOfToken :type Integer))
  (if (>= (Variables|Default|GetcurrentToken) amountOfToken)
    (Variables|Default|SetcurrentToken (- (Variables|Default|GetcurrentToken) amountOfToken))
    (return true)
    (else
      (return false))))

(fn GiveTokenBack
  (params (amountOfToken :type Integer))
  (Variables|Default|SetcurrentToken (+ (Variables|Default|GetcurrentToken) amountOfToken)))