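; Hand enemy Blueprint in the basic AI system whose Range attack is a high-speed charge at the player.
; A montage notify snapshots the player's position from the Blackboard, sets focus and starts AIMoveTo.
; Capsule hits on the player deal damage through a DoOnce, reset each charge.
; Success or failure plays the montage's end section, then fires the attack dispatcher and lowers speed; functions supply per-state speeds and attack/defence radii.
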(event OnComponentHit(CapsuleComponent)
  (params (HitComponent :type Primitive%20Component%20Object%20Reference) (OtherActor :type Actor%20Object%20Reference) (OtherComp :type Primitive%20Component%20Object%20Reference) (NormalImpulse :type Vector :default "0, 0, 0") (Hit :type Hit%20Result%20Structure%20%28by%20ref%29))
  (Utilities|IsValid OtherActor
    (:Is%20Valid
      (if (Actor|ActorHasTag OtherActor "Player")
        (Utilities|FlowControl|DoOnce false
          (:Completed
            (Class|BPIStats|TakeDamage(Message) OtherActor (Utilities|Struct|MakeS_DamageAMK 1e+01 "NewEnumerator0" "NewEnumerator0"))))))))

(event EventBeginPlay)

(event Collision|EventActorBeginOverlap
  (params (OtherActor :type Actor%20Object%20Reference)))

(event EventTick
  (params (DeltaSeconds :type Float%20%28single-precision%29)))

(event EventEnemyAttack
  (params (enemyAttackType :type E_AttackType%20Enum :default "NewEnumerator0"))
  (bind (_returnvalue _aicontroller) (|PlayersPositionGraph))
  (switch Utilities|FlowControl|Switch|SwitchonE_AttackType enemyAttackType
    (:NewEnumerator1
      (Animation|Montage|PlayMontage (Variables|Character|GetMesh) "/Game/NewFolder/fisttransimdat_Montage.fisttransimdat_Montage"
        (:OnNotifyBegin
          (bind _output_get (Variables|Default|SetplayersPosition _returnvalue))
          (AI|SetFocalPoint _aicontroller _output_get)
          (Variables|/Script/Engine.CharacterMovementComponent|SetMaxWalkSpeed (Variables|Character|GetCharacterMovement) 4e+03)
          (AI|AIMoveTo self _output_get 0 25.0 true
            (:then
              (Utilities|FlowControl|DoOnce false) ; enters at Reset
            )
            (:OnSuccess
              (Variables|Default|SetplayersPosition "0, 0, 0" :!label _label)
              (Animation|Montage|PlayMontage (Variables|Character|GetMesh) "/Game/NewFolder/fisttransimdat_Montage.fisttransimdat_Montage" 1.0 0.0 "end"
                (:OnCompleted
                  (Default|CallAttackDispatcher)
                  (Variables|/Script/Engine.CharacterMovementComponent|SetMaxWalkSpeed (Variables|Character|GetCharacterMovement) 2e+02))))
            (:OnFail
              (goto _label))))))))

(fn ConstructionScript
  (|CallParentFunction))

(fn SetMovementSpeed
  (params (movementSpeedEnum :type E_MovementSpeed%20Enum :default "NewEnumerator0"))
  (bind _output_get (Variables|/Script/Engine.CharacterMovementComponent|SetMaxWalkSpeed (Variables|Character|GetCharacterMovement) (Utilities|Select :Index movementSpeedEnum :NewEnumerator0 0.0 :NewEnumerator1 5e+02 :NewEnumerator2 4e+03)))
  (return _output_get))

(fn SetRange
  (return (Utilities|Struct|MakeS_Range 1.2e+02 1.5e+02)))