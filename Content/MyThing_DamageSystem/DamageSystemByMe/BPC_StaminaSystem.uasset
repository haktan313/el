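; BPC_StaminaSystem is a Blueprint component from a damage system that holds and adjusts a current and maximum stamina value.
; DecreaseStamina subtracts an amount only while stamina is above zero and returns whether that depleted it, without clamping the result at zero.
; IncreaseStamina adds an amount and caps the result at MaxStamina.
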(fn DecreaseStamina
  (params (decreaseAmount :type Float%20%28double-precision%29))
  (if (> (Variables|Default|GetcurrentStamina) 0.0)
    (bind _output_get (Variables|Default|SetcurrentStamina (- (Variables|Default|GetcurrentStamina) decreaseAmount)))
    (if (<= _output_get 0.0)
      (return true)
      (else
        (return false)))))

(fn IncreaseStamina
  (params (IncreaseAmount :type Float%20%28double-precision%29))
  (if (<= (Variables|Default|GetcurrentStamina) (Variables|Default|GetmaxStamina))
    (if (<= (+ IncreaseAmount (Variables|Default|GetcurrentStamina)) (Variables|Default|GetmaxStamina))
      (Variables|Default|SetcurrentStamina (+ IncreaseAmount (Variables|Default|GetcurrentStamina)))
      (else
        (Variables|Default|SetcurrentStamina (Variables|Default|GetmaxStamina))))))