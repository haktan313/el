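; Blueprint component that tracks a mana pool, with functions to spend and restore mana.
; DecreaseMana subtracts only while mana is above zero, does not clamp the result, and returns whether that subtraction depleted the pool.
; IncreaseMana adds mana and caps it at MaxMana.
; The event graph is empty, so mana changes only through calls to these functions, with no regeneration over time.
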(event EventBeginPlay)

(event EventTick
  (params (DeltaSeconds :type Float%20%28single-precision%29)))

(fn DecreaseMana
  (params (amount :type Float%20%28double-precision%29))
  (if (> (Variables|Default|GetcurrentMana) 0.0)
    (bind _output_get (Variables|Default|SetcurrentMana (- (Variables|Default|GetcurrentMana) amount)))
    (if (<= _output_get 0.0)
      (return true)
      (else
        (return false)))))

(fn IncreaseMana
  (params (increaseAmount :type Float%20%28double-precision%29))
  (if (<= (Variables|Default|GetcurrentMana) (Variables|Default|GetmaxMana))
    (if (<= (+ increaseAmount (Variables|Default|GetcurrentMana)) (Variables|Default|GetmaxMana))
      (Variables|Default|SetcurrentMana (+ increaseAmount (Variables|Default|GetcurrentMana)))
      (else
        (Variables|Default|SetcurrentMana (Variables|Default|GetmaxMana))))))